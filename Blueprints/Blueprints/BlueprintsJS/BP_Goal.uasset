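; Level goal actor that ends the run when the player ball enters it before timeout.
; On overlap it stops timer, ball and input, then blends from the ball's camera to its own via a timeline.
; Tick polls the Goal component's StartAnimation flag to raise an animated robot, show score calculation, then float it with waves.
; ZoomOnPawn moves the camera to PictureCamera's view, flashes and opens WinningMap.
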(event `self.ReceiveBeginPlay`
  (bind _returnvalue (`GameplayStatics.GetGameMode`))
  (bind _asbp_ball_gamemode (cast `/Game/LevelPrototyping/Blueprints/BlueprintsJS/BP_BallGamemode` _returnvalue))
  (`/Game/LevelPrototyping/Blueprints/BlueprintsJS/BP_BallGamemode.SetGoal` _asbp_ball_gamemode self)
  (bind _asball_game_mode (cast `BallGameMode` _returnvalue))
  (set `BallGameMode.HasFinished` false _asball_game_mode)
  (set `self.IsIn` false)
  (set `self.NewCameraTransform` (`SceneComponent.K2_GetComponentToWorld` (`self.Camera`)))
  (set `self.NewFOV` (`CameraComponent.FieldOfView` (`self.Camera`)))
  (set `GoalComponent.SplashVFX` (`self.NS_Splash`) (`self.Goal`)))

(event `self.Goal.OnComponentBeginOverlap`
  (params (OverlappedComponent :type "PrimitiveComponent Object Reference") (OtherActor :type "Actor Object Reference") (OtherComp :type "PrimitiveComponent Object Reference") (OtherBodyIndex :type Integer) (bFromSweep :type Boolean) (SweepResult :type "HitResult Structure (by ref)"))
  (bind _camera (`self.Camera`))
  (bind _asbp_ball_gamemode (cast `/Game/LevelPrototyping/Blueprints/BlueprintsJS/BP_BallGamemode` (`GameplayStatics.GetGameMode`)))
  (if (and (`self.ActorHasTag` OtherActor "Player") (not (`BallGameMode.IsTimeout` _asbp_ball_gamemode)))
    (if (not (`self.IsIn`))
      (set `self.IsIn` true)
      (bind _asbp_ball_pawn (cast `/Game/LevelPrototyping/Blueprints/BlueprintsJS/BP_Ball_Pawn` OtherActor))
      (`self.RemoveInputs` _asbp_ball_pawn)
      (`self.SetLevelEnding`)
      (`GoalComponent.StopBall` (`self.Goal`) _asbp_ball_pawn)
      (`SizeComponent.BlockInputsAndScale` (`/Game/LevelPrototyping/Blueprints/BlueprintsJS/BP_Ball_Pawn.Size` _asbp_ball_pawn) false)
      (bind _camera_2 (`Ball_Pawn.Camera` _asbp_ball_pawn))
      (set `self.OldCameraTransform` (`SceneComponent.K2_GetComponentToWorld` _camera_2))
      (set `self.OldFOV` (`CameraComponent.FieldOfView` _camera_2))
      (`PlayerController.SetViewTargetWithBlend` (`GameplayStatics.GetPlayerController` 0) self 0.0 "VTBlend_Linear" 0.0 false)
      (bind (_direction _newtrack_0) (`Timeline|ChangeCamera`)
        (:`Update`
          (`SceneComponent.K2_SetWorldTransform` _camera (`KismetMathLibrary.TLerp` (`self.OldCameraTransform`) (`self.NewCameraTransform`) _newtrack_0) false false)
          (`CameraComponent.SetFieldOfView` _camera (`KismetMathLibrary.Lerp` (`self.OldFOV`) (`self.NewFOV`) _newtrack_0))
          (bind _asball_pawn (cast `Ball_Pawn` (`GameplayStatics.GetPlayerPawn` 0)))
          (set `Ball_Pawn.IsPlaying` false _asball_pawn))))))

(event `self.ReceiveTick`
  (params (DeltaSeconds :type "Float (single-precision)"))
  (bind _sm_robot_idle (`self.SM_Robot_Idle`))
  (bind _sm_robot_idle_2 (`self.SM_Robot_Idle`))
  (bind _sm_robot_idle_3 (`self.SM_Robot_Idle`))
  (bind _goal (`self.Goal`))
  (bind (_relativelocation_x _relativelocation_y _relativelocation_z) (`KismetMathLibrary.BreakVector` (`SceneComponent.RelativeLocation` _sm_robot_idle_2)))
  (bind (_relativelocation_x_2 _relativelocation_y_2) (`KismetMathLibrary.BreakVector` (`SceneComponent.RelativeLocation` _sm_robot_idle_3)))
  (if (`GoalComponent.StartAnimation` _goal)
    (set `GoalComponent.StartAnimation` false _goal)
    (`SceneComponent.SetVisibility` _sm_robot_idle true false)
    (`SkeletalMeshComponent.PlayAnimation` _sm_robot_idle "/Game/LevelPrototyping/Animation/Ending/SM_Robot_Closed_Anim.SM_Robot_Closed_Anim" true)
    (bind (_direction _z_position) (`Timeline|MoveToSurface`)
      (:`Update`
        (`SceneComponent.K2_SetRelativeLocation` _sm_robot_idle_3 (`KismetMathLibrary.MakeVector` _relativelocation_x_2 _relativelocation_y_2 _z_position) false false))
      (:`Finished`
        ;[1 1 1] calculate score
        (bind _returnvalue (`|CreateWidget` "/Game/LevelPrototyping/UI/ScoreCalculation/WBP_ScoreCalculation.WBP_ScoreCalculation_C"))
        (`UserWidget.AddToViewport` _returnvalue 0)
        (`SkeletalMeshComponent.PlayAnimation` (`self.SM_Robot_Idle`) "/Game/LevelPrototyping/Animation/SM_Robot_Win_Anim.SM_Robot_Win_Anim" true)
        (bind (_direction_2 _z_position_2) (`Timeline|Floting`)
          (:`Update`
            (`SceneComponent.K2_SetRelativeLocation` _sm_robot_idle_2 (`KismetMathLibrary.MakeVector` _relativelocation_x _relativelocation_y _z_position_2) false false)
            (if (and (not (`ActorComponent.IsActive` (`self.NS_Waves`))) (> _relativelocation_z -120.0))
              (`ActorComponent.Activate` (`self.NS_Waves`) false))))))))

(event `ZoomOnPawn`
  (bind (_direction _newtrack_0) (`Timeline|Timeline`)
    (:`Update`
      (`SceneComponent.K2_SetWorldTransform` (`self.Camera`) (`KismetMathLibrary.TLerp` (`self.NewCameraTransform`) (`SceneComponent.K2_GetComponentToWorld` (`self.PictureCamera`)) _newtrack_0) false false))
    (:`Finished`
      (bind _returnvalue (`|CreateWidget` "/Game/LevelPrototyping/UI/WinningPage/WBP_Flash.WBP_Flash_C"))
      (`UserWidget.AddToViewport` _returnvalue 0)
      (`KismetSystemLibrary.Delay` 0.4)
      (`GameplayStatics.OpenLevel` "WinningMap"))))

(fn `PlaySplash`
  (params (SpawnPosition :type "Vector2D Structure")))

(fn `RemoveInputs`
  (params (self2 :type "Ball_Pawn Object Reference"))
  (`WidgetBlueprintLibrary.SetInputMode_UIOnlyEx` (`GameplayStatics.GetPlayerController` 0) null))

(fn `SetLevelEnding`
  (bind _asball_game_mode (cast `BallGameMode` (`GameplayStatics.GetGameMode`)))
  (if (not (`BallGameMode.HasFinished` _asball_game_mode))
    (set `BallGameMode.HasFinished` true _asball_game_mode)
    (`BallGameMode.StopTimer` _asball_game_mode)))

(fn `UserConstructionScript`)