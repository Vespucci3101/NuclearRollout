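; Player ball pawn Blueprint that supplies sound and VFX for resizing, fans, item placement and attacks.
; BeginPlay hands shockwave effects to the AttackComponent and creates audio components; resize inputs play grow/shrink sounds, which Tick stops at scale limits.
; AddFan and SubFan set a counter that Tick reads, firing a separate 2D cue whenever FanSound is idle; SubFan always zeroes it.
; The emissive material swap is unwired.
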(event `self.CreatingItemEvent`
  (`GameplayStatics.PlaySound2D` "/Game/LevelPrototyping/Music/building_Cue.building_Cue" 1.0 1.0 0.0 null null))

(event `self.NotAbleToPlaceItemEvent`
  (`GameplayStatics.PlaySound2D` "/Game/LevelPrototyping/Music/cant_place_object_here_bucko_Cue.cant_place_object_here_bucko_Cue" 1.0 1.0 0.0 null null))

(event `self.ReceiveBeginPlay`
  (`self.SetVFX` (`self.Attack`))
  (bind _returnvalue (`AddComponent|NODE_AddAudioComponent-3`))
  (bind _output_get (set `self.GrowingSound` _returnvalue))
  (`AudioComponent.SetSound` _output_get "/Game/LevelPrototyping/Music/Growing_cue.Growing_cue")
  (bind _returnvalue_2 (`AddComponent|NODE_AddAudioComponent-4`))
  (bind _output_get_2 (set `self.ShrinkingSound` _returnvalue_2))
  (`AudioComponent.SetSound` _output_get_2 "/Game/LevelPrototyping/Music/Shrinking_cue.Shrinking_cue")
  (bind _returnvalue_3 (`AddComponent|NODE_AddAudioComponent-6`))
  (bind _output_get_3 (set `self.FanSound` _returnvalue_3))
  (`AudioComponent.SetSound` _output_get_3 "/Game/LevelPrototyping/Music/Fan_Fanning_cue.Fan_Fanning_cue")
  (set `self.PassedKillzone` false))

(event `InputAction|IncreaseSize`
  (params (Key :type "Key Structure"))
  (bind _growingsound (`self.GrowingSound`))
  (bind _relativescale3d_x (`KismetMathLibrary.BreakVector` (`SceneComponent.RelativeScale3D` (`self.StaticMesh`))))
  (:`Pressed`
    (if (<= _relativescale3d_x 4.9)
      (`AudioComponent.Play` _growingsound 0.0)))
  (:`Released`
    (`AudioComponent.Stop` _growingsound)))

(event `self.ReceiveTick`
  (params (DeltaSeconds :type "Float (single-precision)"))
  (bind _relativescale3d_x (`KismetMathLibrary.BreakVector` (`SceneComponent.RelativeScale3D` (`self.StaticMesh`))))
  (bind _relativescale3d_x_2 (`KismetMathLibrary.BreakVector` (`SceneComponent.RelativeScale3D` (`self.StaticMesh`))))
  (if (> (`self.Fan`) 0)
    (if (not (`AudioComponent.IsPlaying` (`self.FanSound`)))
      (`GameplayStatics.PlaySound2D` "/Game/LevelPrototyping/Music/Fan_Fanning_cue.Fan_Fanning_cue" 1.0 1.0 0.0 null null))
    (else
      (`AudioComponent.Stop` (`self.FanSound`))))
  (if (not (<= _relativescale3d_x 4.9))
    (`AudioComponent.Stop` (`self.GrowingSound`)))
  (if (not (>= _relativescale3d_x_2 0.81))
    (`AudioComponent.Stop` (`self.ShrinkingSound`))))

(event `InputAction|DecreaseSize`
  (params (Key :type "Key Structure"))
  (bind _shrinkingsound (`self.ShrinkingSound`))
  (bind _relativescale3d_x (`KismetMathLibrary.BreakVector` (`SceneComponent.RelativeScale3D` (`self.StaticMesh`))))
  (:`Pressed`
    (if (>= _relativescale3d_x 0.81)
      (`AudioComponent.Play` _shrinkingsound 0.0)))
  (:`Released`
    (`AudioComponent.Stop` _shrinkingsound)))

(event `InputAction|Attack`
  (params (Key :type "Key Structure"))
  ;[1 1 1] Material emissive
)

(fn `AddFan`
  (bind _result (`/Engine/EditorBlueprintResources/StandardMacros.IncrementInt` (`self.Fan`))
    (:`  `
      (set `self.Fan` _result))))

(fn `SetMat`
  (`PrimitiveComponent.SetMaterial` (`self.StaticMesh`) 0 "/Game/LevelPrototyping/Materials/MI_Reacteur.MI_Reacteur")
  (`PrimitiveComponent.SetMaterial` (`self.StaticMesh`) 1 "/Game/LevelPrototyping/Materials/MI_Chapeau.MI_Chapeau")
  (`PrimitiveComponent.SetMaterial` (`self.StaticMesh`) 2 "/Game/LevelPrototyping/Materials/MI_Cockpit.MI_Cockpit"))

(fn `SetMatNoE`
  (`PrimitiveComponent.SetMaterial` (`self.StaticMesh`) 0 "/Game/LevelPrototyping/Materials/PlayerAttacked/MI_Reacteur_No_Emissive.MI_Reacteur_No_Emissive")
  (`PrimitiveComponent.SetMaterial` (`self.StaticMesh`) 1 "/Game/LevelPrototyping/Materials/PlayerAttacked/MI_Chapeau_No_Emissive.MI_Chapeau_No_Emissive")
  (`PrimitiveComponent.SetMaterial` (`self.StaticMesh`) 1 "/Game/LevelPrototyping/Materials/PlayerAttacked/MI_Cockpit_No_Emissive.MI_Cockpit_No_Emissive"))

(fn `SetVFX`
  (params (Object :type "Object Object Reference"))
  (bind _asattack_component (cast `AttackComponent` Object))
  (set `AttackComponent.Shockwave` (`self.PShockwave`) _asattack_component)
  (set `AttackComponent.GroundShockwave` (`self.PShockwaveGround`) _asattack_component))

(fn `StopBallPawnSFX`
  (`AudioComponent.Stop` (`self.ShrinkingSound`))
  (`AudioComponent.Stop` (`self.GrowingSound`)))

(fn `SubFan`
  (`/Engine/EditorBlueprintResources/StandardMacros.DecrementInt` (`self.Fan`)
    (:`  `
      (set `self.Fan` 0))))

(fn `UserConstructionScript`)