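; Game mode for the ball game that runs the level intro, HUD and lighting-driven time pressure.
; An item selection screen, skipped on Alpha_0, leads to a 3-2-1-Go widget, which then adds the HUD and last-life warning, starts the timer and enables play.
; With 15 seconds left, Tick plays a warning, tints and animates the directional light.
; LightsOutAndStop blocks ball input, kills the lights and ends the level.
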(event `self.ReceiveBeginPlay`)

(event `AddItemsUI`
  (bind _returnvalue (`GameplayStatics.GetCurrentLevelName` true))
  (if (`KismetStringLibrary.EqualEqual_StrStr` _returnvalue "Alpha_0")
    (bind _returnvalue_2 (`|CreateWidget` "/Game/LevelPrototyping/UI/PopUp/WBP_321Go.WBP_321Go_C" :!label _label))
    (add `/Game/LevelPrototyping/UI/PopUp/WBP_321Go.GoFired` _returnvalue_2 (delegate `AddGameplayUI`))
    (`UserWidget.AddToViewport` _returnvalue_2 0)
    (else
      (bind _returnvalue_3 (`|CreateWidget` "/Game/LevelPrototyping/ItemSelection.ItemSelection_C"))
      (add `/Game/LevelPrototyping/ItemSelection.ItemSelected` _returnvalue_3 (delegate `321Go`))
      (`UserWidget.AddToViewport` _returnvalue_3 0))))

(event `321Go`
  (goto _label))

(event `AddGameplayUI`
  (bind _asball_game_instance (cast `BallGameInstance` (`GameplayStatics.GetGameInstance`)))
  (if (== (`BallGameInstance.NumberOfLives` _asball_game_instance) 1)
    (bind _returnvalue (`|CreateWidget` "/Game/LevelPrototyping/UI/PopUp/WBP_LastChance.WBP_LastChance_C"))
    (`UserWidget.AddToViewport` _returnvalue 0)
    (`GameplayStatics.PlaySound2D` "/Game/LevelPrototyping/Music/Annoucer_Last_chance_Cue.Annoucer_Last_chance_Cue" 1.0 1.0 0.0 null null))
  (bind _returnvalue_2 (`|CreateWidget` "/Game/LevelPrototyping/Blueprints/BlueprintsJS/WBP_Timer.WBP_Timer_C"))
  (`UserWidget.AddToViewport` _returnvalue_2 0)
  (bind _returnvalue_3 (`|CreateWidget` "/Game/LevelPrototyping/Blueprints/BlueprintsJS/WBP_Mass.WBP_Mass_C"))
  (`UserWidget.AddToViewport` _returnvalue_3 0)
  (bind _returnvalue_4 (`|CreateWidget` "/Game/LevelPrototyping/Blueprints/BlueprintsJS/WBP_Collectible.WBP_Collectible_C"))
  (`UserWidget.AddToViewport` _returnvalue_4 0)
  (bind _returnvalue_5 (`|CreateWidget` "/Game/LevelPrototyping/Blueprints/BlueprintsJS/WBP_Score.WBP_Score_C"))
  (`UserWidget.AddToViewport` _returnvalue_5 0)
  (bind _returnvalue_6 (`|CreateWidget` "/Game/LevelPrototyping/Blueprints/BlueprintsJS/WBP_Lives.WBP_Lives_C"))
  (`UserWidget.AddToViewport` _returnvalue_6 0)
  (`GameplayStatics.GetCurrentLevelName` true)
  (bind _returnvalue_7 (`|CreateWidget` "/Game/LevelPrototyping/CurrentItem.CurrentItem_C"))
  (`UserWidget.AddToViewport` _returnvalue_7 0)
  (`self.StartTimer`)
  (`WidgetBlueprintLibrary.SetInputMode_GameOnly` (`GameplayStatics.GetPlayerController` 0))
  (bind _asball_pawn (cast `Ball_Pawn` (`GameplayStatics.GetPlayerPawn` 0)))
  (set `Ball_Pawn.IsPlaying` true _asball_pawn))

(event `LightsOutAndStop`
  (bind _outactors (`GameplayStatics.GetAllActorsOfClass` "/Script/Engine.SpotLight"))
  (for _array_element _outactors
    (`LightComponent.SetIntensity` (`SpotLight.SpotLightComponent` _array_element) 0.0))
  (bind _asbp_ball_pawn (cast `/Game/LevelPrototyping/Blueprints/BlueprintsJS/BP_Ball_Pawn` (`GameplayStatics.GetPlayerPawn` 0)))
  (`SizeComponent.BlockInputsAndScale` (`/Game/LevelPrototyping/Blueprints/BlueprintsJS/BP_Ball_Pawn.Size` _asbp_ball_pawn) true)
  (`GameplayStatics.GetAllActorsOfClass` "/Script/Engine.SpotLight")
  (bind _returnvalue (`GameplayStatics.GetActorOfClass` "/Script/Engine.DirectionalLight"))
  (`GameplayStatics.PlaySound2D` "/Game/LevelPrototyping/Music/lights_out_Cue.lights_out_Cue" 1.0 1.0 0.0 null null)
  (bind (_direction _intensity) (`Timeline|ShutLights`)
    (:`Update`
      (`LightComponent.SetIntensity` (`Light.LightComponent` _returnvalue) _intensity))
    (:`Finished`
      (`KismetSystemLibrary.Delay` 0.5)
      (`self.CallEndLevel` false))))

(event `self.ReceiveTick`
  (params (DeltaSeconds :type "Float (single-precision)"))
  (bind _asbp_ball_gamemode (cast `/Blueprints/Blueprints/BlueprintsJS/BP_BallGamemode` (`GameplayStatics.GetGameMode`)))
  (if (and (<= (`BallGameMode.TimeLeft` _asbp_ball_gamemode) 15.0) (not (`self.IsHalfLightTriggered`)))
    (switch `int` (`KismetMathLibrary.RandomIntegerInRange` 0 3)
      (:`0`
        (`GameplayStatics.PlaySound2D` "/Game/LevelPrototyping/Music/time_is_running_out_1_Cue.time_is_running_out_1_Cue" 1.0 1.0 0.0 null null))
      (:`1`
        (`GameplayStatics.PlaySound2D` "/Game/LevelPrototyping/Music/time_is_running_out_2.time_is_running_out_2" 1.0 1.0 0.0 null null)))
    (bind _returnvalue (`GameplayStatics.GetActorOfClass` "/Script/Engine.DirectionalLight"))
    (bind _lightcomponent (`Light.LightComponent` _returnvalue))
    (`LightComponent.SetLightColor` _lightcomponent (`KismetMathLibrary.CInterpTo` (`LightComponentBase.GetLightColor` _lightcomponent) (struct :`R` 1.0 :`G` 0.4 :`B` 0.4 :`A` 1.0) DeltaSeconds 2.0) true)
    (bind (_direction _intensity) (`Timeline|Timeline`)
      (:`Update`
        (`LightComponent.SetIntensity` _lightcomponent _intensity)
        (set `self.IsHalfLightTriggered` true)))))

(fn `SetGoal`
  (params (goal :type "/Game/LevelPrototyping/Blueprints/BlueprintsJS/BP_Goal Object Reference"))
  (set `self.Goal` goal))

(fn `TriggerEventLightsOutAndStop`
  (`self.LightsOutAndStop`))

(fn `UserConstructionScript`)