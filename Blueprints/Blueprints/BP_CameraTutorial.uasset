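; BP_CameraTutorial is a trigger actor that shows the camera tutorial the first time the player overlaps it.
; A flag on BallGameInstance records that the tutorial is done so it does not repeat, with a local IsIn flag as an extra guard.
; On trigger, it adds WBP_CameraTutorial to the viewport, marks the game instance as paused and pauses the game.
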(event `self.ReceiveActorBeginOverlap`
  (params (OtherActor :type "Actor Object Reference"))
  (if (`self.ActorHasTag` OtherActor "Player")
    (bind _asball_game_instance (cast `BallGameInstance` (`GameplayStatics.GetGameInstance`)))
    (if (not (`BallGameInstance.IsCameraTutorialDone` _asball_game_instance))
      (set `BallGameInstance.IsCameraTutorialDone` true _asball_game_instance)
      (if (not (`self.IsIn`))
        (set `self.IsIn` true)
        (set `BallGameInstance.IsGamePaused` true _asball_game_instance)
        (bind _returnvalue (`|CreateWidget` "/Game/LevelPrototyping/UI/PopUp/WBP_CameraTutorial.WBP_CameraTutorial_C"))
        (`UserWidget.AddToViewport` _returnvalue 0)
        (`GameplayStatics.SetGamePaused` true)))))

(fn `UserConstructionScript`)