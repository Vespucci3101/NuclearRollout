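; BP_KillZone is a trigger that stages the player ball's fall to its death.
; On the first overlap by a Player-tagged BP_Ball_Pawn, it plays a dying sound, flags the pawn and switches the view to its own camera, copied from the pawn's transform and FOV.
; Tick then rotates that stationary camera to track the ball and adds downward velocity to speed up the fall, unless StopFollowing is set.
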(event `self.ReceiveActorBeginOverlap`
  (params (OtherActor :type "Actor Object Reference"))
  (bind _asbp_ball_pawn (cast `/Game/LevelPrototyping/Blueprints/BlueprintsJS/BP_Ball_Pawn` OtherActor))
  (if (and (`self.ActorHasTag` OtherActor "Player") (not (`/Game/LevelPrototyping/Blueprints/BlueprintsJS/BP_Ball_Pawn.PassedKillzone` _asbp_ball_pawn)))
    (if (not (`self.HasHit`))
      (set `self.HasHit` true)
      (bind _returnvalue (`GameplayStatics.SpawnSound2D` "/Game/LevelPrototyping/Music/Dieing_Cue.Dieing_Cue" 1.0 1.0 0.0 null))
      (set `self.FallingSound` _returnvalue)
      (`self.ChangeCamera` _asbp_ball_pawn)
      (set `self.ballPawn` _asbp_ball_pawn)
      (set `/Game/LevelPrototyping/Blueprints/BlueprintsJS/BP_Ball_Pawn.PassedKillzone` true _asbp_ball_pawn)
      (set `self.StopFollowing` false))))

(event `self.ReceiveTick`
  (params (DeltaSeconds :type "Float (single-precision)"))
  (bind _ballpawn (`self.ballPawn`))
  (bind _camera (`self.Camera`))
  (if (and (`self.HasHit`) (`KismetSystemLibrary.IsValid` _ballpawn))
    (if (not (`self.StopFollowing`))
      (`SceneComponent.K2_SetWorldRotation` _camera (`KismetMathLibrary.Conv_VectorToRotator` (- (`SceneComponent.K2_GetComponentLocation` (`Ball_Pawn.StaticMesh` _ballpawn)) (`SceneComponent.K2_GetComponentLocation` _camera))) false false)
      (`self.AccelerateBallPawn` DeltaSeconds))))

(fn `AccelerateBallPawn`
  (params (DeltaTime :type "Float (double-precision)"))
  (bind _staticmesh (`Ball_Pawn.StaticMesh` (`self.ballPawn`)))
  (bind _returnvalue (`PrimitiveComponent.GetPhysicsLinearVelocity` _staticmesh "None"))
  (`PrimitiveComponent.SetPhysicsLinearVelocity` _staticmesh (`KismetMathLibrary.MakeVector` (.x _returnvalue) (.y _returnvalue) (- (.z _returnvalue) (* DeltaTime (`self.FallingAcceleration`)))) false "None"))

(fn `ChangeCamera`
  (params (ballPawn :type "/Game/LevelPrototyping/Blueprints/BlueprintsJS/BP_Ball_Pawn Object Reference"))
  (bind _camera (`self.Camera`))
  (bind _camera_2 (`Ball_Pawn.Camera` ballPawn))
  (`SceneComponent.K2_SetWorldTransform` _camera (`SceneComponent.K2_GetComponentToWorld` _camera_2) false false)
  (`CameraComponent.SetFieldOfView` _camera (`CameraComponent.FieldOfView` _camera_2))
  (`PlayerController.SetViewTargetWithBlend` (`GameplayStatics.GetPlayerController` 0) self 0.0 "VTBlend_Linear" 0.0 false)
  (set `Ball_Pawn.SkydomeIsDisabled` true ballPawn))

(fn `UserConstructionScript`)