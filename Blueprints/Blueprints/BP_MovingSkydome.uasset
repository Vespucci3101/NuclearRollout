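; BP_MovingSkydome is a skydome actor with a Death trigger that ends the level as a loss when the player falls into it.
; On BeginPlay it caches the kill zone and ball pawn, and lowers SkyTop on level Alpha_7.
; The first player overlap plays a Niagara splash above the ball, stops the kill zone's following and falling sound, then calls the game mode's CallEndLevel after a delay.
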(event `self.ReceiveBeginPlay`
  (bind _returnvalue (`GameplayStatics.GetActorOfClass` "/Game/LevelPrototyping/Blueprints/BP_KillZone.BP_KillZone_C"))
  (set `self.killZone` _returnvalue)
  (bind _returnvalue_2 (`GameplayStatics.GetActorOfClass` "/Game/LevelPrototyping/Blueprints/BlueprintsJS/BP_Ball_Pawn.BP_Ball_Pawn_C"))
  (set `self.ballPawn` _returnvalue_2)
  (bind _returnvalue_3 (`GameplayStatics.GetCurrentLevelName` true))
  (if (`KismetStringLibrary.EqualEqual_StrStr` _returnvalue_3 "Alpha_7")
    (`SceneComponent.K2_AddLocalOffset` (`self.SkyTop`) (0.0 0.0 -1000.0) false false)
    (set `self.splashPlayed` false)))

(event `self.ReceiveTick`
  (params (DeltaSeconds :type "Float (single-precision)")))

(event `self.Death.OnComponentBeginOverlap`
  (params (OverlappedComponent :type "PrimitiveComponent Object Reference") (OtherActor :type "Actor Object Reference") (OtherComp :type "PrimitiveComponent Object Reference") (OtherBodyIndex :type Integer) (bFromSweep :type Boolean) (SweepResult :type "HitResult Structure (by ref)"))
  (bind _killzone (`self.killZone`))
  (bind _fallingsound (`/Game/LevelPrototyping/Blueprints/BP_KillZone.FallingSound` _killzone))
  (if (and (not (`self.splashPlayed`)) (`self.ActorHasTag` OtherActor "Player"))
    (`self.PlaySplashVFXAtRightPlacement`)
    (`/Engine/EditorBlueprintResources/StandardMacros.IsValid` _killzone
      (:`Is Valid`
        (set `/Game/LevelPrototyping/Blueprints/BP_KillZone.StopFollowing` true _killzone)
        (`/Engine/EditorBlueprintResources/StandardMacros.IsValid` _fallingsound
          (:`Is Valid`
            (`ActorComponent.SetActive` _fallingsound false false))
          (:`Is Not Valid`
            _)))
      (:`Is Not Valid`
        _))
    (`KismetSystemLibrary.Delay` 2.0)
    (bind _asbp_ball_gamemode (cast `/Game/LevelPrototyping/Blueprints/BlueprintsJS/BP_BallGamemode` (`GameplayStatics.GetGameMode`)))
    (`BallGameMode.CallEndLevel` _asbp_ball_gamemode false)))

(fn `PlaySplashVFXAtRightPlacement`
  (bind _ns_deathsplash (`self.NS_DeathSplash`))
  (bind (_returnvalue_x _returnvalue_y _returnvalue_z) (`KismetMathLibrary.BreakVector` (`SceneComponent.K2_GetComponentLocation` (`Ball_Pawn.StaticMesh` (`self.ballPawn`)))))
  (`SceneComponent.K2_SetWorldLocation` _ns_deathsplash (`KismetMathLibrary.MakeVector` _returnvalue_x _returnvalue_y (+ _returnvalue_z 5000.0)) false true)
  (`ActorComponent.Activate` _ns_deathsplash false)
  (set `self.splashPlayed` true))

(fn `UserConstructionScript`)