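; Spring pad Blueprint that launches the ball pawn upward and plays a jump sound when it enters the box trigger.
; The impulse's Z is the pad's up-vector Z times SpringMultiplier and ball mass, while X and Y come from the ball's relative scale.
; A HasBoosted flag blocks repeat boosts until any actor overlap with the pad ends.
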(event `self.Box.OnComponentBeginOverlap`
  (params (OverlappedComponent :type "PrimitiveComponent Object Reference") (OtherActor :type "Actor Object Reference") (OtherComp :type "PrimitiveComponent Object Reference") (OtherBodyIndex :type Integer) (bFromSweep :type Boolean) (SweepResult :type "HitResult Structure (by ref)"))
  (bind (_returnvalue_x _returnvalue_y _returnvalue_z) (`KismetMathLibrary.BreakVector` (* (`self.SpringMultiplier`) (`self.GetActorUpVector`))))
  (bind _asbp_ball_pawn (cast `/Game/LevelPrototyping/Blueprints/BlueprintsJS/BP_Ball_Pawn` OtherActor))
  (if (not (`self.HasBoosted`))
    (set `self.HasBoosted` true)
    (bind (_returnvalue_x_2 _returnvalue_y_2) (`KismetMathLibrary.BreakVector` (`self.GetActorRelativeScale3D` _asbp_ball_pawn)))
    (`PrimitiveComponent.AddImpulse` (`Ball_Pawn.StaticMesh` _asbp_ball_pawn) (`KismetMathLibrary.MakeVector` _returnvalue_x_2 _returnvalue_y_2 (* _returnvalue_z (`PrimitiveComponent.GetMass` (`Ball_Pawn.StaticMesh` _asbp_ball_pawn)))) "None" false)
    (`GameplayStatics.PlaySound2D` "/Game/LevelPrototyping/Music/Ball_Jump_cue.Ball_Jump_cue" 1.0 1.0 0.0 null null)))

(event `self.ReceiveActorEndOverlap`
  (params (OtherActor :type "Actor Object Reference"))
  (set `self.HasBoosted` false))

(fn `UserConstructionScript`)