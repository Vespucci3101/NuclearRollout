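; BP_Fan_2 is a fan actor that pushes BP_Ball_Pawn balls inside its box volume along a configurable force vector.
; The construction script sizes the box from range variables and raises it by its half-height so it sits on the actor origin.
; Each tick, it scans the box's overlapping actors and applies a delta-time-scaled impulse to each ball's static mesh.
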(event `self.ReceiveTick`
  (params (DeltaSeconds :type "Float (single-precision)"))
  (for _array_element (`PrimitiveComponent.GetOverlappingActors` (`self.Box`) null)
    (bind _asbp_ball_pawn (cast `/Game/LevelPrototyping/Blueprints/BlueprintsJS/BP_Ball_Pawn` _array_element))
    (`PrimitiveComponent.AddImpulse` (`Ball_Pawn.StaticMesh` _asbp_ball_pawn) (* DeltaSeconds (`KismetMathLibrary.MakeVector` (`self.ForceX`) (`self.ForceY`) (`self.ForceZ`))) "None" false)))

(fn `UserConstructionScript`
  (bind _box (`self.Box`))
  (bind (_boxextent_x _boxextent_y _boxextent_z) (`KismetMathLibrary.BreakVector` (`BoxComponent.BoxExtent` _box)))
  (`BoxComponent.SetBoxExtent` (`self.Box`) (/ (`KismetMathLibrary.MakeVector` (`self.RangeX`) (`self.RangeY`) (`self.RangeZ`)) (2.0 2.0 2.0)) true)
  (`SceneComponent.K2_SetRelativeLocation` _box (`KismetMathLibrary.MakeVector` 0.0 0.0 _boxextent_z) false false))