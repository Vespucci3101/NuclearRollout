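; BP_Collectible is a pickup that rotates and bobs on a sine wave, unless IsNotMoving is set, which stops both motions.
; Overlap of its capsule by an actor tagged Player sets IsDestroyed and destroys it.
; The Destroyed event checks that flag, then plays a sound, passes the pickup location to the player's BP_Ball_Pawn via CollectCollectible and shows a WBP_ScoreGained widget.
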(event `self.Capsule.OnComponentBeginOverlap`
  (params (OverlappedComponent :type "PrimitiveComponent Object Reference") (OtherActor :type "Actor Object Reference") (OtherComp :type "PrimitiveComponent Object Reference") (OtherBodyIndex :type Integer) (bFromSweep :type Boolean) (SweepResult :type "HitResult Structure (by ref)"))
  (if (`self.ActorHasTag` OtherActor "Player")
    (set `self.IsDestroyed` true)
    (`self.K2_DestroyActor`)))

(event `self.ReceiveDestroyed`
  (if (`self.IsDestroyed`)
    (`GameplayStatics.PlaySound2D` "/Game/LevelPrototyping/Music/nuclear_pickup_cue.nuclear_pickup_cue" 1.0 1.0 0.0 null null)
    (bind _asbp_ball_pawn (cast `/Game/LevelPrototyping/Blueprints/BlueprintsJS/BP_Ball_Pawn` (`GameplayStatics.GetPlayerPawn` 0)))
    (`Ball_Pawn.CollectCollectible` _asbp_ball_pawn (`self.K2_GetActorLocation`))
    (bind _returnvalue (`|CreateWidget` "/Game/LevelPrototyping/UI/PopUp/WBP_ScoreGained.WBP_ScoreGained_C"))
    (`UserWidget.AddToViewport` _returnvalue 0)))

(event `self.ReceiveTick`
  (params (DeltaSeconds :type "Float (single-precision)"))
  (if (`self.IsNotMoving`)
    (set `RotatingMovementComponent.RotationRate` (struct) (`self.RotatingMovement`))
    (else
      (bind _output_get (set `self.T` (+ DeltaSeconds (`self.T`))))
      (`self.K2_AddActorWorldOffset` (`KismetMathLibrary.MakeVector` 0.0 0.0 (* (`KismetMathLibrary.Sin` (* _output_get 5.0)) 0.28))))))

(fn `UserConstructionScript`)