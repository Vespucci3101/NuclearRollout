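; BP_Seesaw is a physics-driven seesaw actor with a Base, a Board and an Axis constraint.
; The Construction Script shifts Axis and Base along local X by OffsetX to place the pivot, scales the Board's mass by SeesawMass, and limits the Axis swing 2 angle to MaxSeesawAngle.
; The Event Graph holds no active logic, so tilting is left to the physics simulation.
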(fn `UserConstructionScript`
  (`SceneComponent.K2_AddLocalOffset` (`self.Axis`) (`KismetMathLibrary.MakeVector` (`self.OffsetX`)) false false)
  (`SceneComponent.K2_AddLocalOffset` (`self.Base`) (`KismetMathLibrary.MakeVector` (`self.OffsetX`)) false false)
  (`PrimitiveComponent.SetMassScale` (`self.Board`) "None" (`self.SeesawMass`))
  (`PhysicsConstraintComponent.SetAngularSwing2Limit` (`self.Axis`) "ACM_Limited" (`self.MaxSeesawAngle`)))